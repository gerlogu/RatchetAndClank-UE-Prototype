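; BP_Bolt is a collectible bolt pickup with looping sequence animation and randomized mesh scale.
; It enables overlap on a custom collision channel shortly after spawning.
; A one-time Pick call waits briefly, awards its value, plays a varied sound and starts a fast looping timer.
; The timer disables physics and pulls the bolt toward the player with rising speed, then a timeline rescales the mesh before destruction.
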(event Custom|Event%20FollowPlayer
  (bind _scale (Variables|Private|GetScale))
  (Physics|SetSimulatePhysics (Variables|Default|GetBox) false)
  (Transformation|SetWorldLocation (Variables|Default|GetBox) (Math|Interpolation|VInterptoConstant (Transformation|GetWorldLocation (Variables|Default|GetBox)) (Transformation|GetActorLocation (Game|GetPlayerCharacter 0)) (* 0.003 3.2) (Variables|Private|GetInterpSpeed)) false false)
  (if (Math|Vector|Equal(Vector) (Transformation|GetWorldLocation (Variables|Default|GetBox)) (Transformation|GetActorLocation (Game|GetPlayerCharacter 0)) 42.0)
    (bind _lerpvalue (Timeline|Timeline_0 Play)
      (:Update
        (Transformation|SetRelativeScale3D (Variables|Default|GetMesh) (Math|Vector|Lerp(Vector) (Math|Vector|MakeVector _scale _scale _scale) "0, 0, 0" _lerpvalue)))
      (:Finished
        (Actor|DestroyActor)))
    (else
      (Variables|Private|SetInterpSpeed (+ (Variables|Private|GetInterpSpeed) 1.7)))))

(event EventBeginPlay
  (bind _returnvalue (Math|Random|RandomFloatinRange 0.7 0.875))
  (Class|MovieSceneSequencePlayer|PlayLooping (Variables|/Script/ActorSequence.ActorSequenceComponent|GetSequencePlayer (Variables|Default|GetActorSequence)) -1)
  (Variables|Private|SetScale _returnvalue)
  (Transformation|SetRelativeScale3D (Variables|Default|GetMesh) (Math|Vector|MakeVector _returnvalue _returnvalue _returnvalue))
  (Utilities|FlowControl|Delay 0.7)
  (Collision|SetCollisionResponsetoChannel (Variables|Default|GetBox) "ECC_GameTraceChannel4" "ECR_Overlap")
  (Variables|Private|SetInterpSpeed (Math|Random|RandomFloatinRange 1.5e+02 2e+02)))

(event EventPick
  (params (Actor :type Actor%20Object%20Reference))
  (if (not (Variables|Private|GetPicked))
    (Variables|Private|SetPicked true)
    (Utilities|FlowControl|Delay (Math|Random|RandomFloatinRange 0.0 0.35))
    (Class|BIBoltPicker|ObtainBolts(Message) Actor (Variables|ExposedonSpawn|GetValue))
    (Audio|PlaySoundatLocation (Utilities|Select :Index (Math|Random|RandomIntegerinRange 0 2) :Option%200 "/Game/GameFiles/Sound/Bolt/Bolt1.Bolt1" :Option%201 "/Game/GameFiles/Sound/Bolt/Bolt3.Bolt3" :Option%202 "/Game/GameFiles/Sound/Bolt/Bolt2.Bolt2") (Transformation|GetWorldLocation (Variables|Default|GetBox)) "0, 0, 0" 1.2 (Math|Random|RandomFloatinRange 0.96 1.04) 0.0 "/Game/GameFiles/Sound/Bolt/SA_Bolt.SA_Bolt" "/Game/GameFiles/Sound/Bolt/SC_Bolt.SC_Bolt" 0)
    (Utilities|Time|SetTimerbyEvent (delegate Custom|Event%20FollowPlayer) 0.003 true)))

(fn ConstructionScript)