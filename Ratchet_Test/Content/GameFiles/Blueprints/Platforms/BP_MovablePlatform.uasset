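; BP_MovablePlatform is a looping moving platform that carries its SuperGridBox between the first two points of its Spline.
; On BeginPlay it scales FollowSplineTimeline's play rate by SpeedMultiplier and plays it from the start, restarting whenever it finishes.
; Each update lerps the box's world location in a straight line between the two points using the timeline's LerpValue, without sweep, so spline curvature is ignored.
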(event EventBeginPlay
  ;[0 0 0] Begin Play
  (Components|Timeline|SetPlayRate (Variables|Default|GetFollowSplineTimeline) (Variables|MovablePlatform|GetSpeedMultiplier))
  (bind _lerpvalue (Timeline|FollowSplineTimeline PlayFromStart)
    (:Update
      (Transformation|SetWorldLocation (Variables|Default|GetSuperGrid_Box) (Math|Vector|Lerp(Vector) (Spline|GetLocationatSplinePoint (Variables|Default|GetSpline) 0 "World") (Spline|GetLocationatSplinePoint (Variables|Default|GetSpline) 1 "World") _lerpvalue) false false))
    (:Finished
      (Components|Timeline|PlayfromStart (Variables|Default|GetFollowSplineTimeline)))))

(fn ConstructionScript)