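; Player controller that sets up game-only input, the HUD and camera pitch limits when play begins.
; On BeginPlay it creates the UI_HUD widget, stores it and adds it to the viewport, then clamps the camera manager's view pitch to a symmetric range.
; GetHUDWidget exposes the stored HUD widget.
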(event EventBeginPlay
  (bind _playercameramanager (Variables|Default|GetPlayerCameraManager))
  (Input|SetInputModeGameOnly self)
  (bind _returnvalue (UserInterface|CreateWidget "/Game/GameFiles/UMG/UI_HUD.UI_HUD_C"))
  (bind _output_get (Variables|Default|SetHUD _returnvalue))
  (UserInterface|Viewport|AddtoViewport _output_get 0)
  (Variables|/Script/Engine.PlayerCameraManager|SetViewPitchMin _playercameramanager -5e+01)
  (Variables|/Script/Engine.PlayerCameraManager|SetViewPitchMax _playercameramanager 5e+01))

(fn ConstructionScript)

(fn GetHUDWidget
  (return (Variables|Default|GetHUD)))