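; BP_LootableBox is a breakable loot box that bursts into bolt pickups when it dies.
; Die spawns the configured quantity of BP_Bolt actors, each carrying the bolt value, at random points and yaws along a spline, then fires a radial force impulse.
; It then swaps the intact cube for a destructible mesh, revealing it, shattering it with radius damage from just below, and destroying the cube component.
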(event EventSpawnBolts
  (params (BoltData :type Bolts%20Data%20Structure))
  (bind _spline (Variables|Default|GetSpline))
  (while (!= (Variables|Default|GetSpawnedBolts) (.quantity BoltData))
    (Math|Integer|IncrementInt (Variables|Default|GetSpawnedBolts)
      (:%20%20
        (Game|SpawnActorfromClass "/Game/GameFiles/Blueprints/Bolts/BP_Bolt.BP_Bolt_C" (Math|Transform|MakeTransform (Spline|GetLocationatDistanceAlongSpline _spline (Math|Random|RandomFloatinRange (Spline|GetDistanceAlongSplineatSplinePoint _spline 0) (Spline|GetDistanceAlongSplineatSplinePoint _spline 2)) "World") (Math|Rotator|MakeRotator 0.0 0.0 (Math|Random|RandomFloatinRange 0.0 3.6e+02)) "1,1,1") "Undefined" 0 (.value BoltData) 0))))
  (Class|RadialForceComponent|FireImpulse (Variables|Default|GetRadialForce)))

(event EventDie
  ;[0 0 0] Event Die
  (CallFunction|SpawnBolts (Variables|Default|GetBoltsData))
  (Rendering|SetVisibility (Variables|Default|GetDestructible) true false)
  (Class|DestructibleComponent|ApplyRadiusDamage (Variables|Default|GetDestructible) 1e+03 (- (Transformation|GetWorldLocation (Variables|Default|GetDestructible)) "0, 0,20.000000") 5e+01 9e+02 true)
  (Components|DestroyComponent (Variables|Default|GetCube)))

(fn ConstructionScript
  (|CallParentFunction))