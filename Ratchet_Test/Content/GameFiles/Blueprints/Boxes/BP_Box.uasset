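; BP_Box is a breakable box that plays a sound when damaged and dies on the first hit.
; TakeDamage looks up its BoxID row in DT_BoxSound, plays that sound with randomized pitch, then calls Die once, guarded by IsDestroyed.
; A missing row only prints an error, so the box does not die.
; The construction script copies the Mesh's first material onto every Destructible slot.
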(event EventTakeDamage
  (params (Damage :type Integer) (Hit :type Hit%20Result%20Structure))
  (bind _min_maxpitchmultiplier (Variables|ReadOnly|Private|GetMin/MaxPitchMultiplier))
  ;[0 0 0] Take Damage
  (bind _returnvalue (Utilities|GetDataTableRow "/Game/GameFiles/DataTables/DT_BoxSound.DT_BoxSound" (.rowname (Variables|ReadOnly|GetBoxID)))
    (:then
      (Audio|PlaySoundatLocation (.Sound (Utilities|Struct|BreakSoundData _returnvalue)) (Transformation|GetWorldLocation (Variables|Default|GetDestructible)) "0, 0, 0" (.Volume (Utilities|Struct|BreakSoundData _returnvalue)) (* (.Pitch (Utilities|Struct|BreakSoundData _returnvalue)) (Math|Random|RandomFloatinRange (.x _min_maxpitchmultiplier) (.y _min_maxpitchmultiplier))) (.StartTime (Utilities|Struct|BreakSoundData _returnvalue)) (.SoundAttenuation (Utilities|Struct|BreakSoundData _returnvalue)) (.SoundConcurreny (Utilities|Struct|BreakSoundData _returnvalue)) 0)
      (if (not (Variables|Status|GetIsDestroyed))
        (Variables|Status|SetIsDestroyed true)
        (CallFunction|Die)))
    (:RowNotFound
      (Utilities|PrintStringAdv "Failing Reading Data Table" true true "(R=1.000000,G=0.098634,B=0.000000,A=1.000000)" 2.0))))

(fn ConstructionScript
  (for (_ _array_index) (Rendering|Material|GetMaterials (Variables|Default|GetDestructible))
    (Rendering|Material|SetMaterial (Variables|Default|GetDestructible) _array_index (Rendering|Material|GetMaterial (Variables|Default|GetMesh) 0))))