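; BP_ExplosiveBox is an explosive crate that starts a fuse when the player hits it, then explodes.
; A looping timer alternates the dynamic material's emissive and test color until the final tick calls Die.
; Die reads the box's DT_ExplosionData row, spawns particles and shatters the destructible with radius damage.
; It then sphere-traces to damage each BI_KillableActor once via interface message and destroys the mesh.
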(event OnComponentHit(Mesh)
  (params (HitComponent :type Primitive%20Component%20Object%20Reference) (OtherActor :type Actor%20Object%20Reference) (OtherComp :type Primitive%20Component%20Object%20Reference) (NormalImpulse :type Vector :default "0, 0, 0") (Hit :type Hit%20Result%20Structure%20%28by%20ref%29))
  ;[0 0 0] On Begin Overlap
  (switch Utilities|FlowControl|Switch|SwitchonECollisionChannel (Collision|GetCollisionObjectType OtherComp)
    (:ECC_GameTraceChannel1
      (if (== (Variables|Status|GetCurrentTicks) -1)
        (Variables|Status|SetCurrentTicks 1)
        (bind _returnvalue (Utilities|Time|SetTimerbyEvent (EventDispatchers|CreateEvent :!event Custom|Event%20PlayExplosionTimer) 0.75 true -0.75))
        (Variables|Status|SetExplosiveTimer _returnvalue)))))

(event Custom|Event%20PlayExplosionTimer
  (bind _currentticks (Variables|Status|GetCurrentTicks))
  ;[0 0 0] Explosion Timer
  (Math|Integer|IncrementInt _currentticks
    (:%20%20
      (if (!= _currentticks 6)
        (|SwapMaterialEffect)
        (else
          (CallFunction|Die))))))

(event EventBeginPlay
  ;[0 0 0] Begin Play
  (|SetupMaterials))

(event EventDie
  ;[0 0 0] Event Die
  (Utilities|Time|ClearandInvalidateTimerbyHandle (Variables|Status|GetExplosiveTimer))
  (|ReadDataTable)
  (Collision|SetCollisionResponsetoChannel (Variables|Character|GetMesh) "ECC_Visibility" "ECR_Ignore")
  (|PlayVisualEffects)
  (Utilities|FlowControl|Sequence
    (:then_0
      (Game|Damage|ApplyDamage))
    (:then_1
      (Components|DestroyComponent (Variables|Character|GetMesh)))))

(fn ConstructionScript
  (|CallParentFunction))