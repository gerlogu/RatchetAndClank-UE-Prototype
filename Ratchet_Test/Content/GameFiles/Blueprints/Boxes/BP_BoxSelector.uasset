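; BP_BoxSelector is a placeable actor that picks which box variant to spawn from a data table.
; Its construction script points the BoxID row handle at DT_BoxSelector and looks up the selected row.
; The row's class is assigned to the BoxActor child actor component, and BoltsData is copied onto the resulting BP_Box.
; The event graph contains no active logic.
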(event EventBeginPlay)

(event Collision|EventActorBeginOverlap
  (params (OtherActor :type Actor%20Object%20Reference)))

(event EventTick
  (params (DeltaSeconds :type Float%20%28single-precision%29)))

(fn ConstructionScript
  (Utilities|Struct|SetmembersinDataTableRowHandle (Variables|BoxSelector|GetBoxID) "/Game/GameFiles/DataTables/DT_BoxSelector.DT_BoxSelector")
  (bind _returnvalue (Utilities|GetDataTableRow "/Game/GameFiles/DataTables/DT_BoxSelector.DT_BoxSelector" (.rowname (Variables|BoxSelector|GetBoxID)))
    (:then
      (ChildActorComponent|SetChildActorClass (Variables|Default|GetBoxActor) (Utilities|Struct|BreakBoxSelector _returnvalue))
      (bind _asbp_box (Utilities|Casting|CastToBP_Box (Variables|/Script/Engine.ChildActorComponent|GetChildActor (Variables|Default|GetBoxActor))))
      (Variables|/Game/GameFiles/Blueprints/Boxes/BP_Box.BP_Box_C|SetBoltsData _asbp_box (Variables|BoxSelector|GetBoltsData)))))