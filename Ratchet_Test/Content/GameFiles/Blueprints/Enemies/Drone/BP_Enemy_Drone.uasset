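; Drone enemy that senses the player and makes ranged attacks, built on a parent enemy class.
; Pawn sensing writes the player to the Blackboard's TargetActor, while attacks use the player character cached at BeginPlay.
; Attack sets the movement state, runs the timed aim-and-shoot montages if a visibility trace hits the player, then resolves movement.
; A separate SpawnBullet event spawns projectiles aimed at the player with EnemyData damage and speed, pending object pooling.
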(event OnSeePawn(PawnSensing)
  (params (Pawn :type Pawn%20Object%20Reference))
  ;[0 0 0] On See Pawn
  (bind _asbp_player_character (Utilities|Casting|CastToBP_PlayerCharacter Pawn))
  (AI|Components|Blackboard|SetValueasObject (AI|GetBlackboard (AI|GetAIController self)) (Utilities|Name|MakeLiteralName "TargetActor") _asbp_player_character))

(event EventBeginPlay
  ;[0 0 0] BeginPlay
  (|CallParentFunction)
  (Variables|Default|SetTarget (Game|GetPlayerCharacter 0)))

(event EventSpawnBullet
  (params (ActorClass :type Actor%20Class%20Reference))
  (bind _enemydata (Variables|Default|GetEnemyData))
  (bind _firepoint (Variables|Default|GetFirePoint))
  (bind (_health _damage _projectilespeed) (Utilities|Struct|BreakEnemyData _enemydata))
  (bind _returnvalue (Transformation|GetWorldLocation _firepoint))
  ;[0 0 0] Spawn Bullet
  (bind _returnvalue_2 (Game|SpawnActorfromClass ActorClass (Math|Transform|MakeTransform _returnvalue (Math|Rotator|FindLookatRotation _returnvalue (Transformation|GetActorLocation (Variables|Default|GetTarget))) "1.000000,0.200000,0.200000") "Undefined" 0 0)) ; This would be replaced by an object pool.
  (Class|BIBullet|SetDamage(Message) _returnvalue_2 _damage)
  (Class|BIBullet|SetSpeed(Message) _returnvalue_2 _projectilespeed))

(event EventAttack
  (params (Index :type Integer))
  ;[0 0 0] Attack
  (Variables|Default|SetMovementState "NewEnumerator2")
  (bind (_outhit _returnvalue) (Collision|LineTraceByChannel (Transformation|GetWorldLocation (Variables|Default|GetFirePoint)) (Transformation|GetActorLocation (Variables|Default|GetTarget)) "TraceTypeQuery1" false 0 "None"))
  (if _returnvalue
    (if (== (.HitActor (Collision|BreakHitResult _outhit)) (Variables|Default|GetTarget))
      (Utilities|BasicAttack)))
  (CallFunction|ResolveMovement))

(fn ConstructionScript
  (|CallParentFunction))

(fn GetMovementState
  (return (Variables|Default|GetMovementState)))