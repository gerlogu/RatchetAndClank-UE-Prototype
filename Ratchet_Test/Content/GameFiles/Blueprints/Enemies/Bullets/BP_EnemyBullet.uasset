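; BP_EnemyBullet is an enemy projectile that deals damage to actors it overlaps.
; The mesh's begin-overlap event sends a TakeDamageMessage to the other actor, then destroys the bullet unless its Damage is -1.
; SetDamage stores the damage value.
; SetSpeed sets the ProjectileMovement initial and max speed, scales its current velocity by that speed and activates the component.
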(event OnComponentBeginOverlap(Mesh)
  (params (OverlappedComponent :type Primitive%20Component%20Object%20Reference) (OtherActor :type Actor%20Object%20Reference) (OtherComp :type Primitive%20Component%20Object%20Reference) (OtherBodyIndex :type Integer) (bFromSweep :type Boolean) (SweepResult :type Hit%20Result%20Structure%20%28by%20ref%29))
  (Class|BIKillableActor|TakeDamage(Message) OtherActor (Variables|Default|GetDamage))
  (if (!= (Variables|Default|GetDamage) -1)
    (Actor|DestroyActor)))

(event EventSetSpeed
  (params (Speed :type Float%20%28single-precision%29))
  (bind _projectilemovement (Variables|Default|GetProjectileMovement))
  (bind _projectilemovement_2 (Variables|Default|GetProjectileMovement))
  (bind _output_get (Variables|/Script/Engine.ProjectileMovementComponent|SetInitialSpeed _projectilemovement Speed))
  (Variables|/Script/Engine.ProjectileMovementComponent|SetMaxSpeed _projectilemovement _output_get)
  (Variables|/Script/Engine.MovementComponent|SetVelocity _projectilemovement_2 (* (Variables|/Script/Engine.MovementComponent|GetVelocity _projectilemovement_2) Speed))
  (Components|Activation|Activate (Variables|Default|GetProjectileMovement) false))

(event EventSetDamage
  (params (Damage :type Integer))
  (Variables|Default|SetDamage Damage))

(fn ConstructionScript)