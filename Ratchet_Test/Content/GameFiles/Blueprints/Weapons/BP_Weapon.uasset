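; BP_Weapon is a weapon actor that takes its owning BP_PlayerCharacter from its parent actor.
; On BeginPlay it binds to that player's OnAttack and OnEndAttack dispatchers, then loads its stats from DT_WeaponData using the DataID row handle into WeaponData.
; A GetPlayer helper returns the cast parent with a success flag.
; The bound attack handlers have no logic in this graph.
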(event EventBindEvents
  ;[0 0 0] Bind Player Event Dispatchers
  (bind _asbp_player_character (Utilities|Casting|CastToBP_PlayerCharacter (Actor|GetParentActor)))
  (EventDispatchers|BindEventtoOnAttack _asbp_player_character (EventDispatchers|CreateEvent :!event Attack))
  (EventDispatchers|BindEventtoOnEndAttack _asbp_player_character (EventDispatchers|CreateEvent :!event EndAttack)))

(event EventBeginPlay
  ;[0 0 0] BeginPlay
  (CallFunction|BindEvents)
  (|LoadDataTable))

(fn ConstructionScript)

(fn GetPlayer
  (bind _returnvalue (Actor|GetParentActor))
  (bind (_asbp_player_character _bsuccess) (Utilities|Casting|CastToBP_PlayerCharacter _returnvalue))
  ;[0 0 0] Get Player
  (return _asbp_player_character _bsuccess))