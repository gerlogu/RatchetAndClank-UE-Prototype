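; Wrench melee weapon for the player, with a three-hit combo, a crouched attack and a boomerang-style throw.
; Attacks broadcast montages; the toggled sphere collider damages each BI_KillableActor once per attack and advances the combo when disabled.
; Throws trace from the camera and use a looping timer to move the wrench along a spline.
; It returns to the hand socket upon reaching the target or hitting an enemy, then reattaches.
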(event OnComponentBeginOverlap(Sphere)
  (params (OverlappedComponent :type Primitive%20Component%20Object%20Reference) (OtherActor :type Actor%20Object%20Reference) (OtherComp :type Primitive%20Component%20Object%20Reference) (OtherBodyIndex :type Integer) (bFromSweep :type Boolean) (SweepResult :type Hit%20Result%20Structure%20%28by%20ref%29))
  ;[0 0 0] Attack Collider Begin Overlap
  (if (and (Utilities|DoesObjectImplementInterface OtherActor "/Game/GameFiles/Blueprints/Interfaces/BI_KillableActor.BI_KillableActor_C") (not (Utilities|Array|ContainsItem (Variables|Private|GetAttackedEnemiesArray) OtherActor)))
    (Utilities|Array|Add (Variables|Private|GetAttackedEnemiesArray) OtherActor)
    (Variables|Private|SetSpeedMultiplier -1.0)
    (Class|BIKillableActor|TakeDamage(Message) OtherActor (.Damage (Utilities|Struct|BreakWeaponData (Variables|Default|GetWeaponData))))))

(event Custom|CustomEvent_0
  (bind _player (CallFunction|GetPlayer))
  (bind _mesh (Variables|/Script/Engine.Character|GetMesh _player))
  (bind _returnvalue (Transformation|GetSocketRotation _mesh "Hand_RSocket"))
  (if (== (Variables|Private|GetSpeedMultiplier) 1.0)
    (bind _output_get (Variables|Private|SetAlpha (+ (Variables|Private|GetAlpha) (* (Variables|Private|GetSpeedMultiplier) 4e+01))))
    (Transformation|SetActorLocationAndRotation (Spline|GetLocationatDistanceAlongSpline (Variables|Default|GetSpline) _output_get "World") (Math|Rotator|MakeRotator 0.0 -9e+01 (.yaw (Spline|GetRotationatDistanceAlongSpline (Variables|Default|GetSpline) _output_get "World"))))
    (if (Math|Vector|Equal(Vector) (Spline|GetLocationatDistanceAlongSpline (Variables|Default|GetSpline) _output_get "World") (Variables|Private|GetTargetLocation) 0.0001)
      (Variables|Private|SetSpeedMultiplier -1.0)
      (else
        (if (Math|Vector|Equal(Vector) (Transformation|GetActorLocation) (Transformation|GetSocketLocation (Variables|/Script/Engine.Character|GetMesh (.Player (CallFunction|GetPlayer))) "Hand_RSocket") 1.0) :!label _label
          (Utilities|Time|ClearandInvalidateTimerbyHandle (Variables|Private|GetTimer))
          (Default|AttachWeapon (.Player (CallFunction|GetPlayer)) true)
          (CallFunction|EnableAttackCollider false false)
          (Transformation|SetActorLocationAndRotation (Transformation|GetSocketLocation _mesh "Hand_RSocket") (Math|Rotator|MakeRotator (.roll _returnvalue) (.pitch _returnvalue) (.yaw _returnvalue)))
          (Variables|Private|SetThroughAttack false)
          (CallFunction|EndMeleeWeaponAttack))))
    (else
      (Transformation|SetActorLocation (Math|Interpolation|VInterptoConstant (Transformation|GetActorLocation) (Transformation|GetSocketLocation (Variables|/Script/Engine.Character|GetMesh (.Player (CallFunction|GetPlayer))) "Hand_RSocket") (* 0.0085 1.1) 3e+03) false false)
      (goto _label))))

(event Custom|ThroughWeapon
  (bind _player (CallFunction|GetPlayer))
  (bind _playercamera (Variables|/Game/GameFiles/Blueprints/Player/BP_PlayerCharacter.BP_PlayerCharacter_C|GetPlayerCamera _player))
  (bind _returnvalue (Transformation|GetWorldLocation _playercamera))
  (Default|AttachWeapon (.Player (CallFunction|GetPlayer)) false)
  (Variables|Private|SetAlpha 0.0)
  (CallFunction|EnableAttackCollider true false)
  (bind _outhit (Collision|LineTraceByChannel _returnvalue (+ _returnvalue (* (Math|Vector|GetForwardVector _playercamera) 1e+04)) "TraceTypeQuery1" false (Utilities|Array|MakeArray _player) "None"))
  (Variables|Private|SetTargetLocation (.Location (Collision|BreakHitResult _outhit)))
  (Variables|Private|SetThroughAttack true)
  (Spline|SetSplinePoints (Variables|Default|GetSpline) (Utilities|Array|MakeArray (Transformation|GetSocketLocation (Variables|/Script/Engine.Character|GetMesh (.Player (CallFunction|GetPlayer))) "Hand_RSocket") (.Location (Collision|BreakHitResult _outhit))) "World" true)
  (Variables|Private|SetSpeedMultiplier 1.0)
  (bind _returnvalue_2 (Utilities|Time|SetTimerbyEvent (delegate Custom|CustomEvent_0) 0.0085 true))
  (Variables|Private|SetTimer _returnvalue_2))

(event Custom|Crouch
  (params (Crouch :type Boolean))
  ;[0 0 0] On Crouch Action
  (Class|BIMovableActor|LockRotation(Message) (.Player (CallFunction|GetPlayer)) Crouch))

(event EventBindEvents
  (bind _player (CallFunction|GetPlayer))
  ;[0 0 0] Bind Events
  (|CallParentFunction)
  (EventDispatchers|BindEventtoOnEndAttackAnimation _player (EventDispatchers|CreateEvent :!event EndMeleeWeaponAttack))
  (EventDispatchers|BindEventtoOnCrouch _player (EventDispatchers|CreateEvent :!event Custom|Crouch)))

(event EventEnableAttackCollider
  (params (Enable :type Boolean) (ResolveMovement :type Boolean))
  ;[0 0 0] Enable Attack Collider
  (Default|CallOnEnableAttackCollider Enable ResolveMovement)
  (if Enable
    (CallFunction|SetCollisionResponse "ECR_Overlap")
    (Audio|PlaySoundatLocation "/Game/GameFiles/Sound/Player/Jump1_Cue.Jump1_Cue" (Transformation|GetWorldLocation (Variables|Default|GetSphere)) "0, 0, 0" 1.2 1.0 0.0 0 0 0)
    (Game|Feedback|PlayDynamicForceFeedback (Game|GetPlayerController 0) 0.145 0.15 true true true true)
    (else
      (CallFunction|SetCollisionResponse "ECR_Ignore")
      (if (not (Variables|Private|GetThroughAttack))
        (Math|Integer|IncrementInt (Variables|Private|GetAttackIndex)
          (:%20%20
            (if (> (Variables|Private|GetAttackIndex) 2)
              (CallFunction|EndMeleeWeaponAttack))))))))

(event EventEndMeleeWeaponAttack
  ;[0 0 0] End Attack
  (Variables|Private|SetAttackIndex 0)
  (Default|CallOnEndAttack))

(event EventAttack
  (params (MovementState :type E_MovementState%20Enum :default "NewEnumerator0"))
  (if (not (Variables|Private|GetThroughAttack))
    (Utilities|Array|Clear (Variables|Private|GetAttackedEnemiesArray))
    (switch Utilities|FlowControl|Switch|SwitchonE_MovementState MovementState
      (:NewEnumerator0
        (Default|CallOnStartAttack (Utilities|Select :Index (Variables|Private|GetAttackIndex) :Option%200 "/Game/GameFiles/Animation/Characters/Ratchet/Ratchet_root_Attack_04_Montage.Ratchet_root_Attack_04_Montage" :Option%201 "/Game/GameFiles/Animation/Characters/Ratchet/Ratchet_root_Attack_02_Montage.Ratchet_root_Attack_02_Montage" :Option%202 "/Game/GameFiles/Animation/Characters/Ratchet/Ratchet_root_Attack_03_Montage.Ratchet_root_Attack_03_Montage") :!label _label))
      (:NewEnumerator1
        (goto _label))
      (:NewEnumerator4
        (Default|CallOnCrouchedAttack "/Game/GameFiles/Animation/Characters/Ratchet/Ratchet_root_CrouchAttack_Montage.Ratchet_root_CrouchAttack_Montage")))))

(event EventBeginPlay
  ;[0 0 0] Event BeginPlay
  (|CallParentFunction)
  (CallFunction|SetCollisionResponse "ECR_Ignore"))

(fn ConstructionScript
  (|CallParentFunction))

(fn SetCollisionResponse
  (params (NewResponse :type ECollisionResponse%20Enum :default "ECR_Ignore"))
  (Collision|SetCollisionResponsetoChannel (Variables|Default|GetSphere) "ECC_WorldDynamic" NewResponse)
  (Collision|SetCollisionResponsetoChannel (Variables|Default|GetSphere) "ECC_PhysicsBody" NewResponse))